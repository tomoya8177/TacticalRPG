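; BP_RandomStage builds a random tile stage from a web service on BeginPlay, and again when D is pressed after destroying existing tiles.
; An async HTTP GET to generateStage with a random integer returns JSON tiles and trees.
; Each tile is spawned, initialized by terrain (Forest becomes deepGrass), and grows trees for matching hexId entries.
; The logged "altitude" is rolled separately from the requested one, and Tiles is never cleared.
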(event EventBeginPlay
  (bind _returnvalue (Math|Random|RandomIntegerinRange 0 1500))
  (bind _returnvalue_2 (Utilities|String|ToString(Integer) _returnvalue))
  (bind _returnvalue_3 (Utilities|String|Append "generateStage/" _returnvalue_2))
  (bind (_url _map) (CallFunction|HttpURLConstructor _returnvalue_3))
  (CallFunction|EnableInput self)
  (Development|PrintString (Utilities|String|Append "setting altitude : " _returnvalue_3) true true "(R=0.000000,G=0.660000,B=1.000000,A=1.000000)" 1e+01)
  (bind _datastring (|AsyncExecuteHTTPGETREQUEST _url _map "" false)
    (:OnSuccess
      (bind _returnvalue_4 (Class|SIOJsonObject|GetObjectArrayField (Class|SIOJsonObject|GetObjectField (Class|SIOJLibrary|ToJsonObject(JsonValue) (Class|SIOJsonValue|ValuefromJsonString _datastring)) "stage") "tiles"))
      (bind _returnvalue_5 (Class|SIOJsonObject|GetObjectArrayField (Class|SIOJsonObject|GetObjectField (Class|SIOJLibrary|ToJsonObject(JsonValue) (Class|SIOJsonValue|ValuefromJsonString _datastring)) "stage") "trees"))
      (for _array_element _returnvalue_4
        (bind _returnvalue_6 (Game|SpawnActorfromClass "/Game/Actors/Stage/terrain/Tile.Tile_C" (Math|Transform|MakeTransform (Math|Vector|MakeVector (Class|SIOJsonObject|GetNumberField (Class|SIOJsonObject|GetObjectField _array_element "position") "x") (Class|SIOJsonObject|GetNumberField (Class|SIOJsonObject|GetObjectField _array_element "position") "y") (Class|SIOJsonObject|GetNumberField (Class|SIOJsonObject|GetObjectField _array_element "position") "z")) "0, 0, 0" "1.000000,1.000000,5.000000") "Undefined" "MultiplyWithRoot" 0 0))
        (bind _output_get (Variables|/Game/Actors/Stage/terrain/Tile.Tile_C|Setid _returnvalue_6 (Math|Float|Truncate (Class|SIOJsonObject|GetNumberField _array_element "id"))))
        (switch string (Class|SIOJsonObject|GetStringField _array_element "terrain")
          (:Default
            (Variables|Default|SetTile%20Type%20Name (Utilities|String|StringToName (Class|SIOJsonObject|GetStringField _array_element "terrain"))))
          (:forest
            (Variables|Default|SetTile%20Type%20Name "deepGrass")))
        (Default|Initialize _returnvalue_6 (Variables|Default|GetTile%20Type%20Name))
        (Utilities|Array|Add (Variables|Default|Gettiles) _returnvalue_6)
        (for _array_element_2 _returnvalue_5
          (if (== (Class|SIOJsonObject|GetNumberField _array_element_2 "hexId") _output_get)
            (Development|PrintString (Utilities|String|Append "tile " (Utilities|String|ToString(Float) (Class|SIOJsonObject|GetNumberField _array_element_2 "hexId")) "should grow tree!!") true true "(R=0.000000,G=0.660000,B=1.000000,A=1.000000)" 1e+01)
            (Default|GrowTree _returnvalue_6)))))))

(event Collision|EventActorBeginOverlap
  (params (OtherActor :type Actor%20Object%20Reference)))

(event EventTick
  (params (DeltaSeconds :type Float%20%28single-precision%29)))

(event Input|KeyboardEvents|D
  (params (Key :type Key%20Structure))
  (bind _returnvalue (Math|Random|RandomIntegerinRange 0 1500))
  (bind _returnvalue_2 (Utilities|String|ToString(Integer) _returnvalue))
  (bind _returnvalue_3 (Utilities|String|Append "generateStage/" _returnvalue_2))
  (bind (_url _map) (CallFunction|HttpURLConstructor _returnvalue_3))
  (:Pressed
    (bind _outactors (Actor|GetAllActorsOfClass "/Game/Actors/Stage/terrain/Tile.Tile_C"))
    (for _array_element _outactors
      (Default|Destroy _array_element))
    (Development|PrintString (Utilities|String|Append "setting altitude : " _returnvalue_3) true true "(R=0.000000,G=0.660000,B=1.000000,A=1.000000)" 1e+01)
    (bind _datastring (|AsyncExecuteHTTPGETREQUEST _url _map "" false)
      (:OnSuccess
        (bind _returnvalue_4 (Class|SIOJsonObject|GetObjectArrayField (Class|SIOJsonObject|GetObjectField (Class|SIOJLibrary|ToJsonObject(JsonValue) (Class|SIOJsonValue|ValuefromJsonString _datastring)) "stage") "tiles"))
        (bind _returnvalue_5 (Class|SIOJsonObject|GetObjectArrayField (Class|SIOJsonObject|GetObjectField (Class|SIOJLibrary|ToJsonObject(JsonValue) (Class|SIOJsonValue|ValuefromJsonString _datastring)) "stage") "trees"))
        (for _array_element_2 _returnvalue_4
          (bind _returnvalue_6 (Game|SpawnActorfromClass "/Game/Actors/Stage/terrain/Tile.Tile_C" (Math|Transform|MakeTransform (Math|Vector|MakeVector (Class|SIOJsonObject|GetNumberField (Class|SIOJsonObject|GetObjectField _array_element_2 "position") "x") (Class|SIOJsonObject|GetNumberField (Class|SIOJsonObject|GetObjectField _array_element_2 "position") "y") (Class|SIOJsonObject|GetNumberField (Class|SIOJsonObject|GetObjectField _array_element_2 "position") "z")) "0, 0, 0" "1.000000,1.000000,5.000000") "Undefined" "MultiplyWithRoot" 0 0))
          (bind _output_get (Variables|/Game/Actors/Stage/terrain/Tile.Tile_C|Setid _returnvalue_6 (Math|Float|Truncate (Class|SIOJsonObject|GetNumberField _array_element_2 "id"))))
          (switch string (Class|SIOJsonObject|GetStringField _array_element_2 "terrain")
            (:Default
              (Variables|Default|SetTile%20Type%20Name (Utilities|String|StringToName (Class|SIOJsonObject|GetStringField _array_element_2 "terrain"))))
            (:forest
              (Variables|Default|SetTile%20Type%20Name "deepGrass")))
          (Default|Initialize _returnvalue_6 (Variables|Default|GetTile%20Type%20Name))
          (Utilities|Array|Add (Variables|Default|Gettiles) _returnvalue_6)
          (for _array_element_3 _returnvalue_5
            (if (== (Class|SIOJsonObject|GetNumberField _array_element_3 "hexId") _output_get)
              (Development|PrintString (Utilities|String|Append "tile " (Utilities|String|ToString(Float) (Class|SIOJsonObject|GetNumberField _array_element_3 "hexId")) "should grow tree!!") true true "(R=0.000000,G=0.660000,B=1.000000,A=1.000000)" 1e+01)
              (Default|GrowTree _returnvalue_6))))))))

(fn ConstructionScript)