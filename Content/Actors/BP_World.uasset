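; BP_World is an actor that builds the game's hex world from server data when play begins.
; It fetches getWorld over an async HTTP GET, parses the JSON and spawns a BP_Hex per tile, choosing its material by terrain.
; It then matches each civilization's hex ID to a tile and spawns a BP_City there, scaled by level.
; An unconnected branch would destroy all hexes and refetch.
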(event EventBeginPlay
  (bind (_url _map) (CallFunction|HttpURLConstructor "getWorld"))
  (CallFunction|EnableInput self)
  (bind _datastring (|AsyncExecuteHTTPGETREQUEST _url _map "" false)
    (:OnSuccess
      (bind _returnvalue (Class|SIOJsonObject|GetObjectArrayField (Class|SIOJLibrary|ToJsonObject(JsonValue) (Class|SIOJsonValue|ValuefromJsonString _datastring)) "tiles"))
      (bind _output_get (Variables|Default|Sethexes _returnvalue))
      (for _array_element _output_get
        (bind _returnvalue_2 (Game|SpawnActorfromClass "/Game/Actors/BP_Hex.BP_Hex_C" (Math|Transform|MakeTransform (Utilities|ObjecttoVector (Class|SIOJsonObject|GetObjectField _array_element "position"))) "Undefined" "MultiplyWithRoot" 0 0))
        (switch string (Class|SIOJsonObject|GetStringField _array_element "terrain")
          (:Default
            (Variables|Default|SetMaterial "/Game/StarterContent/Materials/M_Ground_Grass.M_Ground_Grass"))
          (:grass
            (Variables|Default|SetMaterial "/Game/StarterContent/Materials/M_Ground_Grass.M_Ground_Grass"))
          (:water
            (Variables|Default|SetMaterial "/Game/Materials/WaterSurface.WaterSurface"))
          (:snow
            (Variables|Default|SetMaterial "/Game/Actors/CHARAC_1/Custom__1_.Custom__1_"))
          (:rock
            (Variables|Default|SetMaterial "/Game/StarterContent/Props/Materials/M_Rock.M_Rock"))
          (:forest
            (Variables|Default|SetMaterial "/Game/StarterContent/Materials/M_Ground_GrassDeep.M_Ground_GrassDeep"))
          (:sand
            (Variables|Default|SetMaterial "/Game/StarterContent/Materials/M_Concrete_Grime.M_Concrete_Grime")))
        (Rendering|Material|SetMaterial (Variables|/Game/Actors/BP_Hex.BP_Hex_C|Gethex _returnvalue_2) 1 (Variables|Default|GetMaterial)))
      (bind _returnvalue_3 (Class|SIOJsonObject|GetObjectArrayField (Class|SIOJLibrary|ToJsonObject(JsonValue) (Class|SIOJsonValue|ValuefromJsonString _datastring)) "civilizations"))
      (for _array_element_2 _returnvalue_3
        (for _array_element_3 (Variables|Default|Gethexes)
          (if (== (Class|SIOJsonObject|GetNumberField _array_element_2 "hexId") (Class|SIOJsonObject|GetNumberField _array_element_3 "id"))
            (Game|SpawnActorfromClass "/Game/Actors/Stage/BP_City.BP_City_C" (Math|Transform|MakeTransform (Utilities|ObjecttoVector (Class|SIOJsonObject|GetObjectField _array_element_3 "position")) "0, 0, 0" (Math|Vector|MakeVector (/ (Class|SIOJsonObject|GetNumberField _array_element_2 "level") 4.0) (/ (Class|SIOJsonObject|GetNumberField _array_element_2 "level") 4.0) (/ (Class|SIOJsonObject|GetNumberField _array_element_2 "level") 4.0))) "Undefined" "MultiplyWithRoot" 0 0)))))))

(event Collision|EventActorBeginOverlap
  (params (OtherActor :type Actor%20Object%20Reference)))

(event EventTick
  (params (DeltaSeconds :type Float%20%28single-precision%29)))

(event Input|KeyboardEvents|D
  (params (Key :type Key%20Structure :default "None")))

(fn ConstructionScript)