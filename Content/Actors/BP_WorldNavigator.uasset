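; BP_WorldNavigator is a player-controlled view actor that moves around the world in steps.
; On BeginPlay it becomes the player's view target, enables click events and adds an Enhanced Input mapping context.
; WASD actions shift it along its forward and right vectors, and Q/E rotate its yaw by a set angle.
; After each move, a vertical trace against WorldDynamic objects snaps it just above the hit, or to zero height on a miss.
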(event Input|EnhancedActionEvents|EnhancedInputActionIA_D
  (params (ActionValue :type Boolean) (ElapsedSeconds :type Float%20%28double-precision%29) (TriggeredSeconds :type Float%20%28double-precision%29) (InputAction :type Input%20Action%20Object%20Reference :default "/Game/InputActions/IA_D.IA_D"))
  (CallFunction|Move "D"))

(event Input|EnhancedActionEvents|EnhancedInputActionIA_Q
  (params (ActionValue :type Boolean) (ElapsedSeconds :type Float%20%28double-precision%29) (TriggeredSeconds :type Float%20%28double-precision%29) (InputAction :type Input%20Action%20Object%20Reference :default "/Game/InputActions/IA_Q.IA_Q"))
  (CallFunction|Rotate "Q"))

(event Input|EnhancedActionEvents|EnhancedInputActionIA_E
  (params (ActionValue :type Boolean) (ElapsedSeconds :type Float%20%28double-precision%29) (TriggeredSeconds :type Float%20%28double-precision%29) (InputAction :type Input%20Action%20Object%20Reference :default "/Game/InputActions/IA_E.IA_E"))
  (CallFunction|Rotate "E"))

(event Input|EnhancedActionEvents|EnhancedInputActionIA_A
  (params (ActionValue :type Boolean) (ElapsedSeconds :type Float%20%28double-precision%29) (TriggeredSeconds :type Float%20%28double-precision%29) (InputAction :type Input%20Action%20Object%20Reference :default "/Game/InputActions/IA_A.IA_A"))
  (CallFunction|Move "A"))

(event Input|EnhancedActionEvents|EnhancedInputActionIA_S
  (params (ActionValue :type Boolean) (ElapsedSeconds :type Float%20%28double-precision%29) (TriggeredSeconds :type Float%20%28double-precision%29) (InputAction :type Input%20Action%20Object%20Reference :default "/Game/InputActions/IA_S.IA_S"))
  (CallFunction|Move "S"))

(event Input|EnhancedActionEvents|EnhancedInputActionIA_W
  (params (ActionValue :type Boolean) (ElapsedSeconds :type Float%20%28double-precision%29) (TriggeredSeconds :type Float%20%28double-precision%29) (InputAction :type Input%20Action%20Object%20Reference :default "/Game/InputActions/IA_W.IA_W"))
  (CallFunction|Move "W"))

(event EventBeginPlay
  (bind _returnvalue (Game|GetPlayerController 0))
  (Game|Player|SetViewTargetwithBlend (Game|GetPlayerController 0) self 0.0 "VTBlend_Linear" 0.0 false)
  (Variables|/Script/Engine.PlayerController|SetbEnableClickEvents _returnvalue true)
  (Input|EnableInput _returnvalue)
  (Input|AddMappingContext (PlayerController|LocalPlayerSubsystems|GetEnhancedInputLocalPlayerSubsystem _returnvalue) "/Game/InputActions/NewInputMappingContext.NewInputMappingContext" 0 "(bIgnoreAllPressedKeysUntilRelease=True,bForceImmediately=False,bNotifyUserSettings=False)"))

(event Collision|EventActorBeginOverlap
  (params (OtherActor :type Actor%20Object%20Reference)))

(event EventTick
  (params (DeltaSeconds :type Float%20%28single-precision%29)))

(fn ConstructionScript)

(fn Rotate
  (params (direction :type Name))
  (bind _returnvalue (Transformation|GetActorRotation))
  (bind (_roll _pitch _yaw) (Math|Rotator|BreakRotator _returnvalue))
  (switch name direction
    (:Q
      (LocalVariables|SetadjustmentDirection 1.0))
    (:E
      (LocalVariables|SetadjustmentDirection -1.0)))
  (Transformation|SetActorRotation (Math|Rotator|MakeRotator _roll _pitch (+ _yaw (* (Variables|Default|GetrotationAngle) (LocalVariables|GetadjustmentDirection))))))

(fn Move
  (params (direction :type Name))
  (bind _returnvalue (Transformation|GetActorForwardVector))
  (bind _returnvalue_2 (Transformation|GetActorRightVector))
  (bind _movedistance (Variables|Default|GetmoveDistance))
  (switch name direction
    (:W
      (LocalVariables|SetdirectionVector _returnvalue))
    (:A
      (LocalVariables|SetdirectionVector (* _returnvalue_2 "-1.000000,-1.000000,-1.000000")))
    (:S
      (LocalVariables|SetdirectionVector (* _returnvalue "-1.000000,-1.000000,-1.000000")))
    (:D
      (LocalVariables|SetdirectionVector _returnvalue_2)))
  (Transformation|SetActorLocation (+ (Transformation|GetActorLocation) (* (LocalVariables|GetdirectionVector) (Math|Vector|MakeVector _movedistance _movedistance _movedistance))) false false)
  (CallFunction|AdjustHeight))

(fn AdjustHeight
  (bind _returnvalue (Transformation|GetActorLocation))
  (bind (_x _y) (Math|Vector|BreakVector _returnvalue))
  (bind (_x_2 _y_2) (Math|Vector|BreakVector _returnvalue))
  (bind (_outhit _returnvalue_2) (Collision|LineTraceForObjects (Math|Vector|MakeVector _x_2 _y_2 3e+03) (Math|Vector|MakeVector _x _y -0.0) (Utilities|Array|MakeArray "ObjectTypeQuery2") false 0 "ForDuration"))
  (if _returnvalue_2
    (Transformation|SetActorLocation (+ (.Location (Collision|BreakHitResult _outhit)) "0.000000,0.000000,20.000000") false false)
    (else
      (Transformation|SetActorLocation (.TraceEnd (Collision|BreakHitResult _outhit)) false false))))