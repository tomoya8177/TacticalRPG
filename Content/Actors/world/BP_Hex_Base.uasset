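; BP_Hex_Base is a base hex tile actor that carries an ID and a toggleable focus highlight.
; Initialize reads the "id" number field from a passed data object and stores it truncated to an integer.
; The Focus component is hidden on BeginPlay, and FocusOn and FocusOff show or hide it without propagating to children.
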(event EventBeginPlay
  (Rendering|SetVisibility (Variables|Default|Getfocus) false false))

(event Collision|EventActorBeginOverlap
  (params (OtherActor :type Actor%20Object%20Reference)))

(event EventTick
  (params (DeltaSeconds :type Float%20%28single-precision%29)))

(fn ConstructionScript)

(fn Initialize
  (params (data :type SIO%20Json%20Object%20Object%20Reference))
  (Variables|Default|Setid (Math|Float|Truncate (Class|SIOJsonObject|GetNumberField data "id"))))

(fn Focuson
  (Rendering|SetVisibility (Variables|Default|Getfocus) true false))

(fn FocusOff
  (Rendering|SetVisibility (Variables|Default|Getfocus) false false))