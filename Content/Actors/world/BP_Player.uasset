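; BP_Player is the player's client-side record of profile, credit, stocks, volume settings, characters and equipment, synced with an HTTP backend.
; Initialize reads player JSON and optionally spawns units plus weapon, shield and armor actors, while reloadPlayerData re-fetches fields without respawning.
; Spending money and saving settings post partial JSON through saveDB using the saved token.
; It also posts new characters, leaves rooms and manages audio playback volume.
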(event Custom|reloadPlayerData
  (bind _token (CallFunction|LoadSavedData (Game|GetGameInstance) (Game|GetGameMode)))
  (bind _datastring (|AsyncExecuteHTTPGETREQUEST (.url (CallFunction|HttpURLConstructor (Utilities|String|Append "player/" (Utilities|String|ToString(Integer) (Variables|Default|Getid))) _token)) (.Map (CallFunction|HttpURLConstructor (Utilities|String|Append "player/" (Utilities|String|ToString(Integer) (Variables|Default|Getid))) _token)) "" false)
    (:OnSuccess
      (CallFunction|SaveGame (Game|GetGameMode) (Game|GetGameInstance) (Variables|Default|Getid))
      (CallFunction|Initialize (Class|SIOJsonObject|GetObjectField (Class|SIOJLibrary|ToJsonObject(JsonValue) (Class|SIOJsonValue|ValuefromJsonString _datastring)) "player") true))))

(event Custom|leaveRoom
  (bind _id (Variables|Default|Getid))
  (bind _returnvalue (Utilities|String|ToString(Integer) _id))
  (bind _returnvalue_2 (Utilities|String|Append "room/leave/" _returnvalue))
  (bind (_url _map) (CallFunction|HttpURLConstructor _returnvalue_2))
  (|AsyncExecuteHTTPGETREQUEST _url _map "" false))

(event Custom|postNewCharacter
  (params (data :type SIO%20Json%20Object%20Object%20Reference) (callbackObject :type Object%20Object%20Reference) (callback :type String))
  (bind (_url _map) (CallFunction|HttpURLConstructor "character"))
  (|AsyncExecuteHTTPPOSTREQUEST _url _map (Utilities|Map|MakeMap "data" (Class|SIOJLibrary|ToString(SIOJsonObject) data)) "" false))

(event Custom|saveDB
  (params (data :type SIO%20Json%20Object%20Object%20Reference))
  (bind _token (CallFunction|LoadSavedData (Game|GetGameInstance) (Game|GetGameMode)))
  (if (Utilities|IsValid data)
    (|AsyncExecuteHTTPPOSTREQUEST (.url (CallFunction|HttpURLConstructor (Utilities|String|Append "player/" (Utilities|String|ToString(Integer) (Variables|Default|Getid))) _token)) (.Map (CallFunction|HttpURLConstructor (Utilities|String|Append "player/" (Utilities|String|ToString(Integer) (Variables|Default|Getid))) _token)) (Utilities|Map|MakeMap "data" (Class|SIOJLibrary|ToString(SIOJsonObject) data)) "" false)
    (else
      (CallFunction|Toast "Data not provided"))))

(event EventBeginPlay)

(event Collision|EventActorBeginOverlap
  (params (OtherActor :type Actor%20Object%20Reference)))

(event EventTick
  (params (DeltaSeconds :type Float%20%28single-precision%29)))

(fn ConstructionScript)

(fn CreateNewCharacterData
  (params (unit :type Unit%20BP%20Object%20Reference))
  (bind _result (Default|GetCPforBasicAttribute unit "NewEnumerator0"))
  (bind _result_2 (Default|GetCPforBasicAttribute unit "NewEnumerator3"))
  (bind _result_3 (Default|GetCPforBasicAttribute unit "NewEnumerator1"))
  (bind _returnvalue (Math|Transform|MakeTransform "0, 0, 0"))
  (bind _result_4 (Default|GetCPforBasicAttribute unit "NewEnumerator2"))
  (bind _totalcp (Variables|/Game/Actors/characterBlueprint.characterBlueprint_C|GettotalCP unit))
  (bind _nickname (Variables|/Game/Actors/characterBlueprint.characterBlueprint_C|Getnickname unit))
  (bind _id (Variables|Default|Getid))
  (bind (_location _rotation) (Math|Transform|BreakTransform _returnvalue))
  (bind _dbcharacterstructure (Utilities|Struct|MakeDBCharacterStructure _nickname _totalcp _result _result_3 _result_4 _result_2 0 0.0 "NewEnumerator0" 0.0 0.0 _id))
  (bind _returnvalue_2 (Class|SIOJLibrary|StructtoJsonObject _dbcharacterstructure))
  (Class|SIOJsonObject|SetObjectField _returnvalue_2 "transform" (Class|SIOJLibrary|StructtoJsonObject (Utilities|Struct|MakeunitTransformStructure _location _rotation)))
  (return _returnvalue_2))

(fn DBEquipmenttoActor
  (params (DBEquipmentObject :type SIO%20Json%20Object%20Object%20Reference))
  (bind _returnvalue (Math|Transform|MakeTransform "0, 0, 0"))
  (bind _equipmenttype (CallFunction|EquipmentTypeStringtoEnum (Class|SIOJsonObject|GetStringField DBEquipmentObject "type")))
  (if (Utilities|Enum|Equal(Enum) _equipmenttype "NewEnumerator0")
    (bind _returnvalue_2 (Game|SpawnActorfromClass "/Game/Actors/Character/Weapon.Weapon_C" _returnvalue "Undefined" "MultiplyWithRoot" 0 0))
    (Default|InitializefromDBObject _returnvalue_2 DBEquipmentObject)
    (Default|InitializeWeaponfromJSONObject _returnvalue_2 (Class|SIOJsonObject|GetObjectField DBEquipmentObject "childWeapon"))
    (return _returnvalue_2)
    (elif (Utilities|Enum|Equal(Enum) _equipmenttype "NewEnumerator4")
      (bind _returnvalue_3 (Game|SpawnActorfromClass "/Game/Actors/Character/Shield.Shield_C" _returnvalue "Undefined" "MultiplyWithRoot" 0 0))
      (Default|InitializefromDBObject _returnvalue_3 DBEquipmentObject)
      (Default|InitializeDBShieldObject _returnvalue_3 (Class|SIOJsonObject|GetObjectField DBEquipmentObject "childShield"))
      (return _returnvalue_3)
      (elif (Utilities|Enum|Equal(Enum) _equipmenttype "NewEnumerator1")
        (bind _returnvalue_4 (Game|SpawnActorfromClass "/Game/Actors/Character/Armor.Armor_C" _returnvalue "AlwaysSpawn" "MultiplyWithRoot" 0 0))
        (Default|InitializefromDBObject _returnvalue_4 DBEquipmentObject)
        (Default|InitializefromDBArmorObject _returnvalue_4 (Class|SIOJsonObject|GetObjectField DBEquipmentObject "childArmor"))
        (return _returnvalue_4)))))

(fn SpendMoney
  (params (value :type Float%20%28double-precision%29))
  (bind _output_get (Variables|Default|Setcredit (- (Variables|Default|Getcredit) value)))
  (bind _foundwidgets (Widget|GetAllWidgetsOfClass "/Game/UIWidgets/EquipmentShop.EquipmentShop_C" false))
  (for _array_element _foundwidgets
    (Variables|/Game/UIWidgets/EquipmentShop.EquipmentShop_C|Setcredit _array_element _output_get))
  (bind _returnvalue (Class|SIOJsonObject|ConstructJsonObject))
  (Class|SIOJsonObject|SetNumberField _returnvalue "credit" _output_get)
  (CallFunction|SaveDB _returnvalue)
  (Audio|PlaySound2D "/Game/Audio/purchase.purchase" 1.0 1.0 0.0 0 0))

(fn Initialize
  (params (JSONObject :type SIO%20Json%20Object%20Object%20Reference) (dontSpawnCharacters :type Boolean))
  (Variables|Default|SetshrineStock (Class|SIOJsonObject|GetNumberField JSONObject "shrineStock"))
  (Variables|Default|SethexId (Math|Float|Truncate (Class|SIOJsonObject|GetNumberField JSONObject "hexId")))
  (Variables|Default|Setnickname (Class|SIOJsonObject|GetStringField JSONObject "nickname"))
  (Variables|Default|SetaudioVolume (Class|SIOJsonObject|GetNumberField JSONObject "audioVolume"))
  (Variables|Default|SetsEVolume (Class|SIOJsonObject|GetNumberField JSONObject "sEVolume"))
  (Variables|Default|Setcredit (Class|SIOJsonObject|GetNumberField JSONObject "credit"))
  (Variables|Default|SetfoodStock (Class|SIOJsonObject|GetNumberField JSONObject "foodStock"))
  (Variables|Default|SetmealStock (Class|SIOJsonObject|GetNumberField JSONObject "mealStock"))
  (Variables|Default|SetmaterialStock (Class|SIOJsonObject|GetNumberField JSONObject "materialStock"))
  (Variables|Default|SetdaysToGo (Math|Float|Truncate (Class|SIOJsonObject|GetNumberField JSONObject "daysToGo")))
  (if (not dontSpawnCharacters)
    (bind _returnvalue (Class|SIOJsonObject|GetObjectArrayField JSONObject "characters"))
    (for _array_element _returnvalue
      (bind _returnvalue_2 (Game|SpawnActorfromClass "/Game/Actors/unitBP.unitBP_C" (Math|Transform|MakeTransform "0, 0, 0") "Undefined" "MultiplyWithRoot" 0 0))
      (Default|InitializefromDBCharacterObject _returnvalue_2 _array_element)
      (Utilities|Array|Add (Variables|Default|Getcharacters) _returnvalue_2))
    (bind _returnvalue_3 (Class|SIOJsonObject|GetObjectArrayField JSONObject "equipments"))
    (for _array_element_2 _returnvalue_3
      (bind _equipment (CallFunction|DBEquipmenttoActor _array_element_2))
      (Utilities|Array|Add (Variables|Default|Getequipments) _equipment))))

(fn PlayAudio
  (params (sound :type Sound%20Base%20Object%20Reference))
  (if (Utilities|IsValid (Variables|Default|GetaudioComponent))
    (Audio|Components|Audio|Stop (Variables|Default|GetaudioComponent)))
  (bind _returnvalue (Audio|SpawnSoundatLocation sound "0, 0, 0" "0, 0, 0" (Variables|Default|GetaudioVolume) 1.0 0.0 0 0))
  (Variables|Default|SetaudioComponent _returnvalue))

(fn UpdateAudioVolume
  (params (value :type Float%20%28double-precision%29))
  (bind _audiocomponent (Variables|Default|GetaudioComponent))
  (bind _output_get (Variables|Default|SetaudioVolume value))
  (if (Utilities|IsValid _audiocomponent)
    (Audio|Components|Audio|SetVolumeMultiplier _audiocomponent _output_get :!class /Script/Engine.AudioComponent)))

(fn UpdateSEVolume
  (params (value :type Float%20%28double-precision%29))
  (bind _secomponent (Variables|Default|GetsEComponent))
  (bind _output_get (Variables|Default|SetsEVolume value))
  (if (Utilities|IsValid _secomponent)
    (Audio|Components|Audio|SetVolumeMultiplier _secomponent _output_get :!class /Script/Engine.AudioComponent)))

(fn SavePersonalSetting
  (bind _returnvalue (Class|SIOJsonObject|ConstructJsonObject))
  (Class|SIOJsonObject|SetNumberField _returnvalue "sEVolume" (Variables|Default|GetsEVolume))
  (Class|SIOJsonObject|SetNumberField _returnvalue "audioVolume" (Variables|Default|GetaudioVolume))
  (Class|SIOJsonObject|SetStringField _returnvalue "nickname" (Variables|Default|Getnickname))
  (CallFunction|SaveDB _returnvalue))