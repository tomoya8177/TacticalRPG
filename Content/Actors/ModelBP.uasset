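; ModelBP is a base-style actor that loads a data record by table and ID from the game's HTTP server.
; On BeginPlay it caches the NewGameMode actor to read its HttpServer address.
; Its load event sends an async GET to the server URL built from Table and Id, then parses the JSON "id" back into Id.
; Success and failure are only printed to screen.
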(event Custom|load
  (Development|PrintString "loading")
  (bind _datastring (|AsyncExecuteHTTPGETREQUEST (Utilities|String|Append (Variables|/Game/NewGameMode.NewGameMode_C|GethttpServer (Variables|Default|GetgameModeRef)) (Variables|Default|Gettable) "/" (Utilities|String|ToString(Integer) (Variables|Default|Getid))) (Utilities|Map|MakeMap "" "") "" false)
    (:OnSuccess
      (Variables|Default|Setid (Math|Float|Truncate (Class|SIOJsonObject|GetNumberField (Class|SIOJLibrary|ToJsonObject(JsonValue) (Class|SIOJLibrary|ToJsonValue(String) _datastring)) "id")))
      (Development|PrintString (Utilities|String|Append "Model loaded. ID: " (Utilities|String|ToString(Integer) (Math|Float|Truncate (Class|SIOJsonObject|GetNumberField (Class|SIOJLibrary|ToJsonObject(JsonValue) (Class|SIOJLibrary|ToJsonValue(String) _datastring)) "id"))))))
    (:OnFail
      (Development|PrintString "http request failed"))))

(event EventBeginPlay
  (bind _returnvalue (Actor|GetActorOfClass "/Game/NewGameMode.NewGameMode_C"))
  (Variables|Default|SetgameModeRef _returnvalue))

(event Collision|EventActorBeginOverlap
  (params (OtherActor :type Actor%20Object%20Reference)))

(event EventTick
  (params (DeltaSeconds :type Float%20%28single-precision%29)))

(fn ConstructionScript)