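; Base terrain tile actor for a stage with movement and attack targeting, initialized from JSON with terrain type, position and ID.
; A data table row keyed by terrain supplies walkability, material and movement cost, with cost rising as the tile sits below zero height.
; An overlay plane highlights movable or attackable tiles.
; Clicks and touches on it move the stage's focus to the tile during certain stage UI statuses.
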(event OnInputTouchEnd(Plane)
  (params (FingerIndex :type ETouchIndex%20Enum :default "Touch1") (TouchedComponent :type Primitive%20Component%20Object%20Reference))
  (bind _stageref (Variables|Default|GetstageRef))
  (switch Utilities|FlowControl|Switch|SwitchonstageUIState (Variables|/Game/UIWidgets/StageUI.StageUI_C|GetStatus (Variables|/Game/Actors/BP_StageBase.BP_StageBase_C|GetStageUIWidgetRef _stageref))
    (:NewEnumerator0)
    (:NewEnumerator1)
    (:NewEnumerator2)
    (:NewEnumerator3
      _)
    (:NewEnumerator6
      _)
    (:NewEnumerator4
      _)
    (:NewEnumerator5)
    (:NewEnumerator7
      _)
    (:NewEnumerator8)
    (:NewEnumerator9
      _))
  (Default|MoveFocus _stageref (Transformation|GetActorLocation)))

(event OnClicked(Plane)
  (params (TouchedComponent :type Primitive%20Component%20Object%20Reference) (ButtonPressed :type Key%20Structure))
  (bind _stageref (Variables|Default|GetstageRef))
  (switch Utilities|FlowControl|Switch|SwitchonstageUIState (Variables|/Game/UIWidgets/StageUI.StageUI_C|GetStatus (Variables|/Game/Actors/BP_StageBase.BP_StageBase_C|GetStageUIWidgetRef _stageref))
    (:NewEnumerator0)
    (:NewEnumerator1)
    (:NewEnumerator2)
    (:NewEnumerator3
      _)
    (:NewEnumerator6
      _)
    (:NewEnumerator4
      _)
    (:NewEnumerator5)
    (:NewEnumerator7
      _)
    (:NewEnumerator8)
    (:NewEnumerator9
      _))
  (Default|MoveFocus _stageref (Transformation|GetActorLocation)))

(event Custom|tileClicked
  (bind _stageref (Variables|Default|GetstageRef))
  (switch Utilities|FlowControl|Switch|SwitchonstageUIState (Variables|/Game/UIWidgets/StageUI.StageUI_C|GetStatus (Variables|/Game/Actors/BP_StageBase.BP_StageBase_C|GetStageUIWidgetRef _stageref))
    (:NewEnumerator0)
    (:NewEnumerator1)
    (:NewEnumerator2)
    (:NewEnumerator3
      _)
    (:NewEnumerator6
      _)
    (:NewEnumerator4
      _)
    (:NewEnumerator5)
    (:NewEnumerator7
      _)
    (:NewEnumerator8)
    (:NewEnumerator9
      _))
  (Default|MoveFocus _stageref (Transformation|GetActorLocation)))

(event EventBeginPlay)

(event Collision|EventActorBeginOverlap
  (params (OtherActor :type Actor%20Object%20Reference)))

(event EventTick
  (params (DeltaSeconds :type Float%20%28single-precision%29)))

(fn ConstructionScript
  (bind _returnvalue (Actor|GetActorOfClass "/Game/Actors/BP_StageBase.BP_StageBase_C"))
  (Variables|Default|SetstageRef _returnvalue))

(fn IsWalkable
  (if (Variables|Default|Getwalkable)
    (return true)
    (else
      (return false))))

(fn Destroy
  (Default|CallDestroyed)
  (Actor|DestroyActor))

(fn HighlightAttackable
  (bind _plane (Variables|Default|GetPlane))
  (Rendering|Material|SetMaterial _plane 0 "/Game/Materials/TileHighlightAttackable.TileHighlightAttackable")
  (Rendering|SetVisibility _plane true false))

(fn HighlightMovable
  (bind _plane (Variables|Default|GetPlane))
  (Rendering|SetVisibility _plane true false)
  (Rendering|Material|SetMaterial _plane 0 "/Game/Materials/TileHighlightMovable.TileHighlightMovable"))

(fn GetMovementCost
  (bind _returnvalue (Transformation|GetActorLocation))
  (bind _type (Variables|Default|Gettype))
  (bind _movementcost (Utilities|Struct|BreakTileTypeStructure _type))
  (bind _z (Math|Vector|BreakVector _returnvalue))
  (if (> _z 0.0)
    (return (Math|Float|Max(Float) _movementcost 1.0))
    (else
      (bind _output_get (LocalVariables|SetNewLocalVar (+ _movementcost (* (/ _z 2e+01) -1.0))))
      (return _output_get))))

(fn SetState
  (params (state :type TileState%20Enum :default "NewEnumerator0"))
  (bind _output_get (Variables|Default|Setstate state))
  (if (Utilities|Enum|Equal(Enum) _output_get "NewEnumerator0")
    (Rendering|SetVisibility (Variables|Default|GetPlane) false false)
    (elif (Utilities|Enum|Equal(Enum) _output_get "NewEnumerator1")
      (CallFunction|HighlightMovable))))

(fn GetPos
  (bind _defaultsceneroot (Variables|Default|GetDefaultSceneRoot))
  (bind _returnvalue (Transformation|GetWorldLocation _defaultsceneroot))
  (bind (_x _y _z) (Math|Vector|BreakVector _returnvalue))
  (return (Utilities|Struct|MakePosStructure (Math|Float|Truncate _x) (Math|Float|Truncate _y) _z)))

(fn GetMaterial
  (bind _returnvalue (Utilities|GetDataTableRow "/Game/DataTables/TileTypeDefinitions.TileTypeDefinitions" (Variables|Default|GettileType))
    (:then
      (bind _output_get (Variables|Default|Settype _returnvalue))
      (return (.material (Utilities|Struct|BreakTileTypeStructure _output_get))))))

(fn Initialize
  (params (data :type SIO%20Json%20Object%20Object%20Reference))
  (bind _output_get (Variables|Default|SettileType (Utilities|String|StringToName (Class|SIOJsonObject|GetStringField data "terrain"))))
  (bind _returnvalue (Utilities|GetDataTableRow "/Game/DataTables/TileTypeDefinitions.TileTypeDefinitions" _output_get)
    (:then
      (bind _output_get_2 (Variables|Default|Settype _returnvalue))
      (Transformation|SetActorLocation (CallFunction|JSONObjecttoVector (Class|SIOJsonObject|GetObjectField data "position")) false true)
      (Variables|Default|Setid (Math|Float|Truncate (Class|SIOJsonObject|GetNumberField data "id")))
      (Variables|Default|Setwalkable (.walkable (Utilities|Struct|BreakTileTypeStructure _output_get_2))))))