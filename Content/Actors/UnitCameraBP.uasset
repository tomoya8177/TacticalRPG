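; Unit camera actor that glides to a target unit's position while its spring arm swings between two view angles.
; A looping timer started on BeginPlay alternates the arm's goal yaw through a FlipFlop, and a timeline blends the rotation along the shortest path.
; setTarget stores the unit and uses a second timeline to lerp the actor to the location that unit had when called.
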(event Custom|setTarget
  (params (unit :type Unit%20BP%20Object%20Reference))
  (Variables|Default|SetstartLocation (Transformation|GetActorLocation))
  (Variables|Default|SetgoalLocation (Transformation|GetActorLocation unit))
  (Variables|Default|SettargetUnit unit)
  (bind _newtrack_0 (Timeline|Timeline PlayFromStart)
    (:Update
      (Transformation|SetActorLocation (Math|Vector|Lerp(Vector) (Variables|Default|GetstartLocation) (Variables|Default|GetgoalLocation) _newtrack_0) false false))))

(event Custom|float
  (Variables|Default|SetstartRotation (Variables|/Script/Engine.SceneComponent|GetRelativeRotation (Variables|Default|GetSpringArm)))
  (Utilities|FlowControl|FlipFlop
    (:A
      (Variables|Default|SetgoalRotation (Math|Rotator|MakeRotator 0.0 -2e+01 -6e+01))
      (bind _newtrack_0 (Timeline|Timeline_0 PlayFromStart)
        (:Update
          (Transformation|SetRelativeRotation (Variables|Default|GetSpringArm) (Math|Rotator|Lerp(Rotator) (Variables|Default|GetstartRotation) (Variables|Default|GetgoalRotation) _newtrack_0 true) false false))))
    (:B
      (Variables|Default|SetgoalRotation (Math|Rotator|MakeRotator 0.0 -2e+01 -1.2e+02))
      (Timeline|Timeline_0 PlayFromStart))))

(event EventBeginPlay
  (Utilities|Time|SetTimerbyEvent (delegate Custom|float) (Variables|Default|GetTime) true)
  (CallFunction|Float))

(event Collision|EventActorBeginOverlap
  (params (OtherActor :type Actor%20Object%20Reference)))

(event EventTick
  (params (DeltaSeconds :type Float%20%28single-precision%29)))

(fn ConstructionScript)