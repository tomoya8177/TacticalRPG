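; Character unit for a tile-based, turn-based tactics game, with tabletop-RPG-style stats derived from attributes and character points.
; Computes skill levels with default fallbacks, movement, encumbrance, damage and dodge/parry/block, using gear from its child EquipmentController.
; Loads its state, equipment and transform from an HTTP JSON backend and saves point and wait-time changes back.
; Clicks pass to the Stage tile beneath, while direction cones send turn requests to the child ActionController.
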(event OnClicked(unitPawn)
  (params (TouchedComponent :type Primitive%20Component%20Object%20Reference) (ButtonPressed :type Key%20Structure))
  (bind _returnvalue (Transformation|GetActorLocation))
  (bind (_x _y _z) (Math|Vector|BreakVector _returnvalue))
  (bind _returnvalue_2 (Actor|GetActorOfClass "/Game/Actors/Stage.Stage_C"))
  (bind _tile (Default|GetTile _returnvalue_2 _x _y _z))
  (Default|TileClicked _tile))

(event OnClicked(West)
  (params (TouchedComponent :type Primitive%20Component%20Object%20Reference) (ButtonPressed :type Key%20Structure))
  (Default|EmitTurnDirection (Variables|Default|GetactionControllerRef) "NewEnumerator0"))

(event OnClicked(East)
  (params (TouchedComponent :type Primitive%20Component%20Object%20Reference) (ButtonPressed :type Key%20Structure))
  (Default|EmitTurnDirection (Variables|Default|GetactionControllerRef) "NewEnumerator1"))

(event OnClicked(North)
  (params (TouchedComponent :type Primitive%20Component%20Object%20Reference) (ButtonPressed :type Key%20Structure))
  (Default|EmitTurnDirection (Variables|Default|GetactionControllerRef) "NewEnumerator2"))

(event Custom|updateFromDB
  (bind (_url _map) (CallFunction|HttpURLConstructor (Utilities|String|Append "character/" (Utilities|String|ToString(Integer) (Variables|Default|Getid)))))
  (bind _datastring (|AsyncExecuteHTTPGETREQUEST _url _map "" false)
    (:OnSuccess
      (if (Class|SIOJsonObject|GetBoolField (Class|SIOJLibrary|ToJsonObject(JsonValue) (Class|SIOJsonValue|ValuefromJsonString _datastring)) "result")
        (Class|SIOJsonObject|GetObjectArrayField (Class|SIOJsonObject|GetObjectField (Class|SIOJLibrary|ToJsonObject(JsonValue) (Class|SIOJsonValue|ValuefromJsonString _datastring)) "character") "equipments")
        (CallFunction|InitializefromDBCharacterObject (Class|SIOJsonObject|GetObjectField (Class|SIOJLibrary|ToJsonObject(JsonValue) (Class|SIOJsonValue|ValuefromJsonString _datastring)) "character"))))))

(event EventBeginPlay)

(event Collision|EventActorBeginOverlap
  (params (OtherActor :type Actor%20Object%20Reference)))

(event EventTick
  (params (DeltaSeconds :type Float%20%28single-precision%29)))

(fn ConstructionScript
  (bind _asaction_controller (Utilities|Casting|CastToActionController (Variables|/Script/Engine.ChildActorComponent|GetChildActor (Variables|Default|GetActionController))))
  (Variables|Default|SetactionControllerRef _asaction_controller)
  (bind _asequipment_controller (Utilities|Casting|CastToEquipmentController (Variables|/Script/Engine.ChildActorComponent|GetChildActor (Variables|Default|GetEquipmentController))))
  (Variables|Default|SetequipmentControllerRef _asequipment_controller)
  (bind _asprompt_controller (Utilities|Casting|CastToPromptController (Variables|/Script/Engine.ChildActorComponent|GetChildActor (Variables|Default|GetPromptController))))
  (Variables|Default|SetpromptControllerRef _asprompt_controller))

(fn GetSkillLevel
  (params (skillName :type Name) (noFollow :type Boolean))
  (bind _returnvalue (Utilities|GetDataTableRow "/Game/DataTables/SkillDefinitions.SkillDefinitions" skillName)
    (:then
      (bind _cp (CallFunction|GetCPforSkill skillName))
      (if (< _cp 0.5)
        (if (.noDefault (Utilities|Struct|BreakSkillStructure _returnvalue))
          (return 0.0)
          (else
            (bind _value (CallFunction|GetBasicAttribute (.attribute (Utilities|Struct|BreakDefaultAttributeStructure (.defaultAttributes (Utilities|Struct|BreakSkillStructure _returnvalue))))))
            (if noFollow
              (return (+ _value (.value (Utilities|Struct|BreakDefaultAttributeStructure (.defaultAttributes (Utilities|Struct|BreakSkillStructure _returnvalue))))))
              (else
                (bind _level (CallFunction|GetSkillLevel (.skillName (Utilities|Struct|BreakDefaultSkillStructure (.fallbackSkill (Utilities|Struct|BreakSkillStructure _returnvalue)))) true))
                (return (Math|Float|Max(Float) (+ _value (.value (Utilities|Struct|BreakDefaultAttributeStructure (.defaultAttributes (Utilities|Struct|BreakSkillStructure _returnvalue))))) (+ _level (.value (Utilities|Struct|BreakDefaultSkillStructure (.fallbackSkill (Utilities|Struct|BreakSkillStructure _returnvalue)))))))))))
        (else
          (bind _value_2 (CallFunction|GetSkillLevelfromCPandDifficulty (.Difficulty (Utilities|Struct|BreakSkillStructure _returnvalue)) _cp (.type (Utilities|Struct|BreakSkillStructure _returnvalue))))
          (return _value_2))))))

(fn GetMovement
  (bind _returnvalue (CallFunction|GetBasicSpeed))
  (bind _value (CallFunction|GetEncumbrance))
  (bind _returnvalue_2 (CallFunction|IsReeling))
  (if _returnvalue_2
    (return (/ (- _returnvalue _value) 2.0))
    (else
      (return (- _returnvalue _value)))))

(fn GetHT
  (bind _value (CallFunction|GetMaxHT))
  (return (- _value (Variables|Default|Getdamage))))

(fn GetCurrentHP
  (bind _value (CallFunction|GetMaxHP))
  (return (- _value (* (Variables|Default|Getdamage) 1e+01))))

(fn InitializefromDBCharacterObject
  (params (DBCharacterObject :type SIO%20Json%20Object%20Object%20Reference))
  (CallFunction|SetPropertiesfromDBObject DBCharacterObject)
  (Rendering|SetVisibility (Variables|Default|GetDirectionCones) false true)
  (CallFunction|InitializeEquipments DBCharacterObject)
  (CallFunction|SetTransform (Class|SIOJsonObject|GetObjectField DBCharacterObject "transform"))
  (CallFunction|InitializeCharacterPanel))

(fn RemoveStatus
  (params (NewParam :type CharacterStates%20Enum :default "NewEnumerator0"))
  (Utilities|Array|RemoveItem (Variables|Default|Getstates) NewParam)
  (return))

(fn GetWT
  (bind _value (CallFunction|GetIQ))
  (bind _value_2 (CallFunction|GetDX))
  (return (/ 1e+02 (+ _value _value_2))))

(fn GetBasicSpeed
  (bind _value (CallFunction|GetMaxDX))
  (bind _value_2 (CallFunction|GetMaxHT))
  (return (/ (+ _value _value_2) 4.0)))

(fn AddDamage
  (params (value :type Float%20%28double-precision%29))
  (Variables|Default|Setdamage (+ value (Variables|Default|Getdamage))))

(fn UseWT
  (params (value :type Float%20%28double-precision%29))
  (Variables|Default|SetcurrentWT (- (Variables|Default|GetcurrentWT) value)))

(fn ShowDirectionCones
  (Rendering|SetVisibility (Variables|Default|GetDirectionCones) true true))

(fn HideDirectionCones
  (Rendering|SetVisibility (Variables|Default|GetDirectionCones) false true))

(fn GetBasicDamage
  (params (attackType :type AttackType%20Enum :default "NewEnumerator0"))
  (if (Utilities|Enum|Equal(Enum) attackType "NewEnumerator0")
    (bind _power (CallFunction|GetPower))
    (return "" _power)
    (elif (Utilities|Enum|Equal(Enum) attackType "NewEnumerator1")
      (bind _power_2 (CallFunction|GetPower))
      (return "" (* _power_2 2.0)))))

(fn GetViewRange
  (return 1.8e+02))

(fn GetEyeLocation
  (bind _defaultsceneroot (Variables|Default|GetDefaultSceneRoot))
  (bind _returnvalue (Transformation|GetWorldLocation _defaultsceneroot))
  (bind (_x _y _z) (Math|Vector|BreakVector _returnvalue))
  (return (Math|Vector|MakeVector _x _y (+ _z 165.0))))

(fn GetDodge
  (bind _value (Default|GetPassiveDiffence (Variables|Default|GetequipmentControllerRef)))
  (bind _movement (CallFunction|GetMovement))
  (return (+ _value _movement)))

(fn GetParries
  (bind _value (Default|GetPassiveDiffence (Variables|Default|GetequipmentControllerRef)))
  (bind _weapons (Default|GetAvailableWeapons (Variables|Default|GetequipmentControllerRef)))
  (for _array_element _weapons
    (if (Variables|/Game/Actors/Character/Weapon.Weapon_C|GetcanParry _array_element)
      (bind _defencestructure (CallFunction|GetParry _value _array_element))
      (Utilities|Array|Add (LocalVariables|Getparries) _defencestructure)))
  (return (LocalVariables|Getparries)))

(fn GetBlocks
  (params (attackFrom :type AttackFrom%20Enum :default "NewEnumerator0"))
  (bind _returnvalue (Utilities|Enum|Equal(Enum) attackFrom "NewEnumerator3"))
  (bind _level (CallFunction|GetSkillLevel "shield" false))
  (bind _shields (Default|GetAvailableShields (Variables|Default|GetequipmentControllerRef)))
  (for _array_element _shields
    (switch string (Variables|/Game/Actors/Character/Equipment.Equipment_C|GetequippedOn _array_element)
      (:RIGHTHAND
        (if (not (or (Utilities|Enum|Equal(Enum) attackFrom "NewEnumerator1") _returnvalue)) :!label _label
          (bind _defencestructure (CallFunction|GetBlock _array_element _level :!label _label_2))
          (Utilities|Array|Add (LocalVariables|GetavailableBlocks) _defencestructure)))
      (:RIGHTARM
        (goto _label))
      (:LEFTHAND
        (if (not (or (Utilities|Enum|Equal(Enum) attackFrom "NewEnumerator2") _returnvalue)) :!label _label_3
          (goto _label_2)))
      (:LEFTARM
        (goto _label_3))
      (:BOTHHAND
        (goto _label_2))
      (:BACK
        (if _returnvalue
          (goto _label_2)))))
  (return (LocalVariables|GetavailableBlocks)))

(fn SetPromptControllerRef)

(fn UseTaskPoint
  (params (pointToConsume :type Float%20%28double-precision%29))
  (bind _output_get (Variables|Default|SettaskPoint (- (Variables|Default|GettaskPoint) pointToConsume)))
  (bind _returnvalue (Class|SIOJsonObject|ConstructJsonObject))
  (Class|SIOJsonObject|SetNumberField _returnvalue "taskPoint" _output_get)
  (CallFunction|SaveDB _returnvalue))

(fn GetEncumbrance
  (CallFunction|GetMaxST)
  (bind _weight (Default|GetWeightSum (Variables|Default|GetequipmentControllerRef)))
  (if (Math|Float|InRange(Float) (Math|Float|Max(Float) (- _weight 1e+01) 0.0) 0.0 3e+01)
    (LocalVariables|Setfactor 0.1)
    (return (* (Math|Float|Max(Float) (- _weight 1e+01) 0.0) (LocalVariables|Getfactor)))
    (elif (Math|Float|InRange(Float) (Math|Float|Max(Float) (- _weight 1e+01) 0.0) 3e+01 1e+02)
      (LocalVariables|Setfactor 0.03)
      (return (* (Math|Float|Max(Float) (- _weight 1e+01) 0.0) (LocalVariables|Getfactor)))
      (elif (Math|Float|InRange(Float) (Math|Float|Max(Float) (- _weight 1e+01) 0.0) 1e+02 5e+02)
        (LocalVariables|Setfactor 0.02)
        (return (* (Math|Float|Max(Float) (- _weight 1e+01) 0.0) (LocalVariables|Getfactor)))))))

(fn IsAlive
  (bind _value (CallFunction|GetCurrentHP))
  (return (> _value 0.0)))

(fn Die
  (bind _returnvalue (Actor|GetActorOfClass "/Game/Actors/Stage.Stage_C"))
  (bind _ismine (CallFunction|IsMine))
  (if _ismine
    (CallFunction|DeletefromDB))
  (for _array_element (Variables|Default|Getequipments)
    (Actor|DestroyActor _array_element))
  (Utilities|Array|RemoveItem (Variables|/Game/Actors/Stage.Stage_C|Getunits _returnvalue) self)
  (Actor|DestroyActor))

(fn ToJsonString
  (bind _outjsonstring (|StructtoJsonString (Utilities|Struct|MakeDBCharacterStructure (Variables|Default|Getnickname) (Variables|Default|GettotalCP) (Variables|Default|GetCPForST) (Variables|Default|GetCPForDX) (Variables|Default|GetCPForIQ) (Variables|Default|GetCPForHT) (Variables|Default|GetCPForSkills) (Variables|Default|Getdamage) (Variables|Default|Getstates) (Variables|Default|GetcurrentWT) (Variables|Default|GettaskPoint) (Variables|Default|GetplayerId) (Variables|Default|Getid))))
  (return _outjsonstring))

(fn RemovefromRoomDB
  (bind _returnvalue (Class|SIOJsonObject|ConstructJsonObject))
  (Class|SIOJsonObject|SetNumberField _returnvalue "roomid" 0.0)
  (CallFunction|SaveDB _returnvalue))

(fn SaveWT
  (bind _returnvalue (Class|SIOJsonObject|ConstructJsonObject))
  (bind _wt (CallFunction|GetWT))
  (Class|SIOJsonObject|SetNumberField _returnvalue "currentWT" _wt)
  (CallFunction|SaveDB _returnvalue))

(fn SetBaseColor
  (params (team :type Integer))
  (if (== team 0)
    (Rendering|Material|SetMaterial (Variables|Default|GetunitPawn) 0 "/Game/Materials/characterBaseBlue.characterBaseBlue")
    (else
      (Rendering|Material|SetMaterial (Variables|Default|GetunitPawn) 0 "/Game/Materials/characterBaseRed.characterBaseRed"))))

(fn UseMovementPoint
  (params (pointToConsume :type Float%20%28double-precision%29))
  (bind _output_get (Variables|Default|SetmovementPoint (- (Variables|Default|GetmovementPoint) pointToConsume)))
  (bind _returnvalue (Class|SIOJsonObject|ConstructJsonObject))
  (Class|SIOJsonObject|SetNumberField _returnvalue "movementPoint" _output_get)
  (CallFunction|SaveDB _returnvalue))

(fn SetTransform
  (params (JSONObject :type SIO%20Json%20Object%20Object%20Reference))
  (bind _transform (CallFunction|TransformJSONtoTransform JSONObject))
  (Transformation|SetActorTransform self _transform)
  (if (>= (Utilities|Array|FindItem (Variables|Default|Getstates) "NewEnumerator1") 0)
    (Transformation|SetRelativeTransform (Variables|Default|GetunitPawn) (Math|Transform|MakeTransform "0.000000,45.000000,40.000000" "0.000000,0.000000,-90.000000") false false)
    (else
      (Transformation|SetRelativeTransform (Variables|Default|GetunitPawn) (Math|Transform|MakeTransform "0, 0, 0") false false))))

(fn GetPower
  (bind _value (CallFunction|GetST))
  (return (Math|Float|Max(Float) (- (* _value 0.5) 3.5) 0.0)))

(fn GetParry
  (params (passiveDefence :type Float%20%28double-precision%29) (weapon :type Weapon%20Object%20Reference))
  (if (Variables|/Game/Actors/Character/Weapon.Weapon_C|GetcanParry weapon)
    (bind _level (CallFunction|GetSkillLevel (Variables|/Game/Actors/Character/Weapon.Weapon_C|GetskillToUse weapon) false))
    (return (Utilities|Struct|MakeDefenceStructure weapon (+ passiveDefence (/ _level 2.0))))
    (else
      (return (Utilities|Struct|MakeDefenceStructure weapon 0.0)))))

(fn GetBlock
  (params (shield :type Equipment%20Object%20Reference) (skillLv :type Float%20%28double-precision%29))
  (bind _value (Default|GetPassiveDiffence (Variables|Default|GetequipmentControllerRef)))
  (return (Utilities|Struct|MakeDefenceStructure shield (+ (/ skillLv 2.0) _value))))

(fn IsReeling
  (bind _value (CallFunction|GetHT))
  (return (<= _value 3.0)))

(fn InitializeEquipments
  (params (DBObject :type SIO%20Json%20Object%20Object%20Reference))
  (bind _equipmentcontrollerref (Variables|Default|GetequipmentControllerRef))
  (bind _returnvalue (Class|SIOJsonObject|GetObjectArrayField DBObject "equipments"))
  (for _array_element _returnvalue
    (bind _equipment (Default|GetEquipmentbyId _equipmentcontrollerref (Math|Float|Truncate (Class|SIOJsonObject|GetNumberField _array_element "id"))))
    (if (Utilities|IsValid _equipment)
      (Default|AttachEquipment _equipmentcontrollerref (Variables|Default|GetcharacterMesh) _equipment)
      (Default|InitializefromDBObject _equipment _array_element)
      (else
        (bind _equipment_2 (Default|DBEquipmenttoActor _equipmentcontrollerref _array_element))
        (Utilities|Array|Add (Variables|Default|Getequipments) _equipment_2)))))

(fn CheckUnconscious
  (bind _value (CallFunction|GetMaxHT))
  (bind _returnvalue (CallFunction|Check _value))
  (return _returnvalue))

(fn InitializeCharacterPanel
  (bind _foundwidgets (Widget|GetAllWidgetsOfClass "/Game/UIWidgets/CharacterPanel.CharacterPanel_C" false))
  (for _array_element _foundwidgets
    (if (and (Utilities|IsValid _array_element) (Utilities|IsValid (Variables|/Game/UIWidgets/CharacterPanel.CharacterPanel_C|Getunit _array_element)))
      (if (== (Variables|Default|Getid) (Variables|/Game/Actors/characterBlueprint.characterBlueprint_C|Getid (Variables|/Game/UIWidgets/CharacterPanel.CharacterPanel_C|Getunit _array_element)))
        (Default|Initialize _array_element)))))