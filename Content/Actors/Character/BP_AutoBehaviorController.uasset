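; Turn-based AI actor that plays turns for its parent unit when it is CPU-controlled or set to auto.
; DecideAction picks the first eligible enemy, attacks if it is in range, otherwise moves or double-moves, or ends the turn.
; Goal search widens the movement budget, tests tiles with a temporary unit clone, and trims the path to available points.
; After moving it turns toward the target; completed turns and attacks trigger another decision.
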(event Custom|unitInTurnSet_Event
  (params (unitId :type Integer))
  (bind _unitref (Variables|Default|GetunitRef))
  (if (== (Variables|/Game/Actors/characterBlueprint.characterBlueprint_C|Getid _unitref) unitId)
    (if (Default|IsMine _unitref)
      (if (Default|IsAuto _unitref)
        (Utilities|FlowControl|Delay 1.5 :!label _label)
        (CallFunction|DecideAction))
      (elif (Default|IsCP _unitref)
        (goto _label)))))

(event Custom|settingTurnDirection_Event
  (bind _actiontarget (Variables|Default|GetactionTarget))
  (bind _unitref (Variables|Default|GetunitRef))
  (bind _returnvalue (Transformation|GetActorTransform _unitref))
  (bind _returnvalue_2 (Transformation|GetActorLocation _actiontarget))
  (bind _actioncontrollerref (Variables|/Game/Actors/unitBP.unitBP_C|GetactionControllerRef _unitref))
  (bind _returnvalue_3 (Math|Rotator|FindRelativeLookatRotation _returnvalue _returnvalue_2))
  (bind _yaw (Math|Rotator|BreakRotator _returnvalue_3))
  (if (Math|Float|InRange(Float) _yaw -45.0 45.0 false false)
    (Default|EmitTurnDirection _actioncontrollerref "NewEnumerator1")
    (elif (or (Math|Float|InRange(Float) _yaw 135.0 1.8e+02) (Math|Float|InRange(Float) _yaw -1.8e+02 -135.0 true false))
      (Default|EmitTurnDirection _actioncontrollerref "NewEnumerator0")
      (elif (Math|Float|InRange(Float) _yaw -135.0 -45.0)
        (Default|EmitTurnDirection _actioncontrollerref "NewEnumerator2")
        (else
          (Default|SetStageUIStatus (Variables|/Game/Actors/BP_StageBase.BP_StageBase_C|GetStageUIWidgetRef (Variables|Default|GetstageRef)) "NewEnumerator4")
          (EventDispatchers|UnbindEventfromSettingTurnDirection _actioncontrollerref (delegate Custom|settingTurnDirection_Event))
          (Utilities|FlowControl|Delay 1.0)
          (CallFunction|DecideAction))))))

(event Custom|assignTurnListener
  (EventDispatchers|AssignSettingTurnDirection (Variables|/Game/Actors/unitBP.unitBP_C|GetactionControllerRef (Variables|Default|GetunitRef)) (delegate Custom|settingTurnDirection_Event)))

(event Custom|assignAttackCompleted
  (params (attackController :type Attack%20Controller%20Object%20Reference))
  (EventDispatchers|AssignAttackCompleted attackController (delegate Custom|attackCompleted_Event)))

(event Custom|attackCompleted_Event
  (Utilities|FlowControl|Delay 1.0)
  (EventDispatchers|UnbindEventfromAttackCompleted (stale Custom|assignAttackCompleted attackController) (delegate Custom|attackCompleted_Event))
  (CallFunction|DecideAction))

(event EventBeginPlay
  (bind _asunit_bp (Utilities|Casting|CastTounitBP (Actor|GetParentActor)))
  (Variables|Default|SetunitRef _asunit_bp)
  (bind _returnvalue (Actor|GetActorOfClass "/Game/Actors/BP_StageBase.BP_StageBase_C"))
  (bind _output_get (Variables|Default|SetstageRef _returnvalue))
  (if (Utilities|IsValid _output_get)
    (EventDispatchers|AssignUnitinTurnSet _output_get (delegate Custom|unitInTurnSet_Event))))

(event Collision|EventActorBeginOverlap
  (params (OtherActor :type Actor%20Object%20Reference)))

(event EventTick
  (params (DeltaSeconds :type Float%20%28single-precision%29)))

(fn ConstructionScript)

(fn LookforTarget
  (for _array_element (Variables|/Game/Actors/BP_StageBase.BP_StageBase_C|Getunits (Variables|Default|GetstageRef))
    (if (and (!= (Variables|/Game/Actors/characterBlueprint.characterBlueprint_C|GetplayerId (Variables|Default|GetunitRef)) (Variables|/Game/Actors/characterBlueprint.characterBlueprint_C|GetplayerId _array_element)) (!= (Default|HasState _array_element "NewEnumerator1") true))
      (return _array_element))))

(fn LookforGoalTile
  (params (targetIn :type Unit%20BP%20Object%20Reference))
  (bind _unitref (Variables|Default|GetunitRef))
  (bind _returnvalue (Default|GetMovementPoint _unitref))
  (bind _output_get (LocalVariables|Settarget targetIn))
  (while (and (!= (Utilities|IsValid (.endTile (Utilities|Struct|BreakPathStructure (LocalVariables|GetpathForFurtherestAndattackable)))) true) (LocalVariables|GetwhileLoopOn))
    (bind _output_get_2 (LocalVariables|SetmultiplyFactor (+ (LocalVariables|GetmultiplyFactor) 0.5)))
    (if (> _output_get_2 2.0)
      (LocalVariables|SetwhileLoopOn false)
      (else
        (Development|PrintString (Utilities|String|Append (Utilities|String|ToString(Float) 0.0) "th trial") true true "(R=0.000000,G=0.660000,B=1.000000,A=1.000000)" 1e+01)
        (bind (_resultpaths1 _unattackabletiles _closestpath1) (CallFunction|FindAttackableTilewithGivenMP (* _returnvalue (LocalVariables|GetmultiplyFactor)) _output_get (LocalVariables|GetunattackableTiles)))
        (if (Utilities|IsValid (.endTile (Utilities|Struct|BreakPathStructure _resultpaths1)))
          (LocalVariables|SetpathForFurtherestAndattackable _resultpaths1)
          (else
            (LocalVariables|SetunattackableTiles _unattackabletiles))))))
  (if (Utilities|IsValid (.endTile (Utilities|Struct|BreakPathStructure (LocalVariables|GetpathForFurtherestAndattackable))))
    _
    (else
      (LocalVariables|SetpathForFurtherestAndattackable _closestpath1)))
  (if (> (.MPToConsume (Utilities|Struct|BreakPathStructure (LocalVariables|GetpathForFurtherestAndattackable))) _returnvalue)
    (for _array_element (.movements (Utilities|Struct|BreakPathStructure (LocalVariables|GetpathForFurtherestAndattackable)))
      (bind _output_get_3 (LocalVariables|SetaccumlatedMP (+ (LocalVariables|GetaccumlatedMP) (.MPToConsume (Utilities|Struct|BreakMovementStructure _array_element)))))
      (if (> _output_get_3 _returnvalue)
        (Development|PrintString (Utilities|String|Append (Utilities|String|ToString(Float) _output_get_3) " out of " (Utilities|String|ToString(Float) _returnvalue)) true true "(R=0.000000,G=0.660000,B=1.000000,A=1.000000)" 1e+01)
        (return (Utilities|Struct|MakePathStructure (LocalVariables|Getmovements) (.endTile (Utilities|Struct|BreakMovementStructure _array_element)) _output_get_3))
        (else
          (Utilities|Array|Add (LocalVariables|Getmovements) _array_element))))
    (else
      (return (LocalVariables|GetpathForFurtherestAndattackable)))))

(fn CheckTargetAttackable
  (params (target :type Unit%20BP%20Object%20Reference) (attacker :type Unit%20BP%20Object%20Reference))
  (bind _stageref (Variables|Default|GetstageRef))
  (bind _attackcontrollerref (Variables|/Game/Actors/BP_StageBase.BP_StageBase_C|GetattackControllerRef _stageref))
  (bind _rangefinderref (Variables|/Game/Actors/BP_StageBase.BP_StageBase_C|GetrangeFinderRef _stageref))
  (LocalVariables|SettargetIn target)
  (if (Variables|Default|GetiCanAttack)
    (bind _weapons (Default|GetAvailableWeapons (Variables|/Game/Actors/unitBP.unitBP_C|GetequipmentControllerRef attacker) false))
    (Default|InitiateAttack _attackcontrollerref attacker (Utilities|Array|Get(acopy) _weapons))
    (Default|FindTilesinRange _rangefinderref false)
    (for _array_element (Variables|/Game/Actors/Stage/RangeFinder.RangeFinder_C|GetattackableTiles _rangefinderref)
      (bind (_unit _result) (Default|GetUnitonTile _stageref _array_element))
      (if _result
        (if (== _unit (LocalVariables|GettargetIn))
          (return true _attackcontrollerref)))))
  (return false 0))

(fn CheckWeaponReady
  (bind _weapons (Default|GetAvailableWeapons (Variables|/Game/Actors/unitBP.unitBP_C|GetequipmentControllerRef (Variables|Default|GetunitRef)) true))
  (return (> (Utilities|Array|Length _weapons) 0)))

(fn DecideAction
  (bind _unitref (Variables|Default|GetunitRef))
  (bind _actioncontrollerref (Variables|/Game/Actors/unitBP.unitBP_C|GetactionControllerRef _unitref))
  (switch int (Math|Float|Truncate (Variables|/Game/Actors/characterBlueprint.characterBlueprint_C|GettaskPoint (Variables|Default|GetunitRef)))
    (:Default
      (Default|EndTurn _actioncontrollerref :!label _label))
    (:0
      (goto _label))
    (:1
      (CallFunction|SetAttackIntension :!label _label_2)
      (CallFunction|SetMoveorRunIntension)
      (bind _target (CallFunction|LookforTarget))
      (if (Utilities|IsValid _target)
        (bind _output_get (LocalVariables|SettargetUnit _target))
        (Variables|Default|SetactionTarget _output_get)
        (if (Utilities|IsValid (Variables|Default|GetactionTarget))
          (bind (_attackable _attackcontroller) (CallFunction|CheckTargetAttackable (Variables|Default|GetactionTarget) (Variables|Default|GetunitRef)))
          (if _attackable
            (Default|FindTilesinRange (Variables|/Game/Actors/BP_StageBase.BP_StageBase_C|GetrangeFinderRef (Variables|Default|GetstageRef)) true)
            (Default|SetTarget _attackcontroller (Variables|Default|GetactionTarget))
            (Default|Execute _attackcontroller)
            (CallFunction|AssignAttackCompleted _attackcontroller)
            (elif (Variables|Default|GetiCanMove)
              (if (Variables|Default|GetiCanRun)
                (bind _dodoublemove (CallFunction|DecideifDoDoubleMove (Variables|Default|GetactionTarget)))
                (if _dodoublemove
                  (Variables|/Game/Actors/Character/ActionController.ActionController_C|SetisDoubleMove _actioncontrollerref true)
                  (else
                    (Variables|/Game/Actors/Character/ActionController.ActionController_C|SetisDoubleMove _actioncontrollerref false :!label _label_3)))
                (else
                  (goto _label_3)))
              (bind _outputpin (CallFunction|LookforGoalTile (Variables|Default|GetactionTarget)))
              (Default|Move _actioncontrollerref _outputpin)
              (CallFunction|AssignTurnListener)
              (else
                (goto _label))))
          (else
            (goto _label)))
        (else
          (goto _label))))
    (:2
      (goto _label_2))
    (:3
      (goto _label_2))))

(fn DecideifDoDoubleMove
  (params (target :type Unit%20BP%20Object%20Reference))
  (bind _unitref (Variables|Default|GetunitRef))
  (bind _weapons (Default|GetAvailableWeapons (Variables|/Game/Actors/unitBP.unitBP_C|GetequipmentControllerRef _unitref) false))
  (if (Utilities|IsValid (Utilities|Array|Get(acopy) _weapons))
    (return (> (- (- (Transformation|GetDistanceTo target _unitref) (Default|GetMovementwithSkillBonus _unitref)) (Variables|/Game/Actors/Character/Weapon.Weapon_C|Getreach (Utilities|Array|Get(acopy) _weapons))) 0.0))
    (else
      (return false))))

(fn SetMoveorRunIntension
  (switch int (Math|Float|Truncate (Variables|/Game/Actors/characterBlueprint.characterBlueprint_C|GetmovementTaskPoint (Variables|Default|GetunitRef)))
    (:Default
      _)
    (:0
      (Variables|Default|SetiCanMove false)
      (Variables|Default|SetiCanRun false))
    (:1
      (Variables|Default|SetiCanMove true)
      (Variables|Default|SetiCanRun false))
    (:2
      (Variables|Default|SetiCanMove true)
      (Variables|Default|SetiCanRun true)))
  (return))

(fn SetAttackIntension
  (bind _weapons (Default|GetAvailableWeapons (Variables|/Game/Actors/unitBP.unitBP_C|GetequipmentControllerRef (Variables|Default|GetunitRef)) false))
  (Variables|Default|SetiCanAttack (> (Utilities|Array|Length _weapons) 0))
  (return))

(fn FindAttackableTilewithGivenMP
  (params (movementPointIn :type Float%20%28double-precision%29) (target :type Unit%20BP%20Object%20Reference) (unattackableTilesSoFar :type Array%20of%20BP%20Tile%20Base%20Object%20References))
  (bind _unitref (Variables|Default|GetunitRef))
  (LocalVariables|SettargetIn target)
  (bind _paths (Default|FindPaths (Variables|/Game/Actors/BP_StageBase.BP_StageBase_C|GetpathFinderRef (Variables|Default|GetstageRef)) (Transformation|GetActorLocation _unitref) (Default|GetCurrentFacingDirection (Variables|/Game/Actors/unitBP.unitBP_C|GetactionControllerRef _unitref)) movementPointIn))
  (for _array_element _paths
    (bind _output_get (LocalVariables|SetpathInQuestion _array_element))
    (if (Utilities|IsValid (.endTile (Utilities|Struct|BreakPathStructure _output_get)))
      (if (>= (Utilities|Array|FindItem unattackableTilesSoFar (.endTile (Utilities|Struct|BreakPathStructure _output_get))) 0)
        (Development|PrintString "This tile is tested that you can't attack from here.")
        (elif (> (Transformation|GetDistanceTo (.endTile (Utilities|Struct|BreakPathStructure _output_get)) (LocalVariables|GettargetIn)) (LocalVariables|GetFarDistance))
          (bind _output_get_2 (LocalVariables|SetdistanceToTarget (Transformation|GetDistanceTo (.endTile (Utilities|Struct|BreakPathStructure _output_get)) (LocalVariables|GettargetIn))))
          (if (< _output_get_2 (LocalVariables|GetclosestDistance))
            (LocalVariables|SetclosestDistance _output_get_2)
            (LocalVariables|SetclosestPath (LocalVariables|GetpathInQuestion)))
          (bind _returnvalue (Class|C3KBPGeneralFL|CloneActor (Variables|Default|GetunitRef)))
          (bind _output_get_3 (LocalVariables|SetcloneUnit _returnvalue))
          (Transformation|SetActorLocationAndRotation _output_get_3 (Transformation|GetActorLocation (.endTile (Utilities|Struct|BreakPathStructure _output_get))) (Math|Rotator|MakeRotator 0.0 0.0 (- (.Yaw (Math|Rotator|BreakRotator (Math|Rotator|FindLookatRotation (Transformation|GetActorLocation (.endTile (Utilities|Struct|BreakPathStructure _output_get))) (Transformation|GetActorLocation (LocalVariables|GettargetIn))))) 9e+01)))
          (bind _attackable (CallFunction|CheckTargetAttackable (LocalVariables|GettargetIn) _output_get_3))
          (Actor|DestroyActor _output_get_3)
          (if _attackable
            (LocalVariables|SetFarDistance (LocalVariables|GetdistanceToTarget))
            (LocalVariables|SetresultPath (LocalVariables|GetpathInQuestion))
            (else
              (Utilities|Array|Add (LocalVariables|GetunattackableTilesTemp) (.endTile (Utilities|Struct|BreakPathStructure _output_get)))))))))
  (return (LocalVariables|GetresultPath) (LocalVariables|GetunattackableTilesTemp) (LocalVariables|GetclosestPath)))