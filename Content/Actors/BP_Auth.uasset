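; Actor that signs a returning player in from saved credentials and spawns their player Blueprint.
; Auth loads the saved player ID and token, then sends an HTTP GET to the player endpoint.
; A positive JSON result saves the refreshed token and broadcasts the player data; dispatchers also report rejection or missing save data.
; A separate event spawns BP_Player at the origin, initializes it from supplied JSON and announces it.
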(event Custom|auth
  (bind _returnvalue (Game|GetGameMode))
  (bind _returnvalue_2 (Game|GetGameInstance))
  (bind (_playerid _result _token) (CallFunction|LoadSavedData _returnvalue_2 _returnvalue))
  (if _result
    (bind _datastring (|AsyncExecuteHTTPGETREQUEST (.url (CallFunction|HttpURLConstructor (Utilities|String|Append "player/" (Utilities|String|ToString(Integer) _playerid)) _token)) (.Map (CallFunction|HttpURLConstructor (Utilities|String|Append "player/" (Utilities|String|ToString(Integer) _playerid)) _token)) "" false)
      (:OnSuccess
        (Development|PrintString "Hello")
        (if (Class|SIOJsonObject|GetBoolField (Class|SIOJLibrary|ToJsonObject(JsonValue) (Class|SIOJsonValue|ValuefromJsonString _datastring)) "result")
          (CallFunction|SaveGame _returnvalue _returnvalue_2 (Math|Float|Truncate (Class|SIOJsonObject|GetNumberField (Class|SIOJsonObject|GetObjectField (Class|SIOJLibrary|ToJsonObject(JsonValue) (Class|SIOJsonValue|ValuefromJsonString _datastring)) "player") "id")) (Class|SIOJsonObject|GetStringField (Class|SIOJLibrary|ToJsonObject(JsonValue) (Class|SIOJsonValue|ValuefromJsonString _datastring)) "newAccessToken"))
          (Variables|Default|SetplayerId (Math|Float|Truncate (Class|SIOJsonObject|GetNumberField (Class|SIOJsonObject|GetObjectField (Class|SIOJLibrary|ToJsonObject(JsonValue) (Class|SIOJsonValue|ValuefromJsonString _datastring)) "player") "id")))
          (Default|CallAuthSuccess (Class|SIOJsonObject|GetObjectField (Class|SIOJLibrary|ToJsonObject(JsonValue) (Class|SIOJsonValue|ValuefromJsonString _datastring)) "player"))
          (else
            (Default|CallAuthFailed)))))
    (else
      (Default|CallNoSaveData))))

(event Custom|spawnPlayerBP
  (params (data :type SIO%20Json%20Object%20Object%20Reference) (dontSpawnCharacters :type Boolean))
  (Development|PrintString "Spawining Player BP")
  (bind _returnvalue (Game|SpawnActorfromClass "/Game/Actors/world/BP_Player.BP_Player_C" (Math|Transform|MakeTransform "0, 0, 0") "Undefined" "MultiplyWithRoot" 0 0))
  (Variables|/Game/Actors/world/BP_Player.BP_Player_C|Setid _returnvalue (Variables|Default|GetplayerId))
  (Default|Initialize _returnvalue data dontSpawnCharacters)
  (Default|CallPlayerBPSpawned _returnvalue))

(event EventBeginPlay)

(event Collision|EventActorBeginOverlap
  (params (OtherActor :type Actor%20Object%20Reference)))

(event EventTick
  (params (DeltaSeconds :type Float%20%28single-precision%29)))

(fn ConstructionScript)